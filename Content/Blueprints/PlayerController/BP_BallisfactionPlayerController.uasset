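; Player controller for Ballisfaction that drives the player pawn with physics-based movement.
; On possession it caches the pawn as BP_BallisfactionPlayer and adds the default Enhanced Input mapping context.
; While move input triggers, it rotates the 2D input by the control rotation's yaw and applies it as a large, mass-dependent force to the pawn's static mesh, giving camera-relative movement.
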(event `self.ReceivePossess`
  (params (PossessedPawn :type "Pawn Object Reference"))
  (bind _asbp_ballisfaction_player (cast `/Game/Blueprints/Player/BP_BallisfactionPlayer` PossessedPawn))
  (set `self.As BP Ballisfaction Player` _asbp_ballisfaction_player)
  (message `EnhancedInputSubsystemInterface.AddMappingContext` (pcsubsystem `EnhancedInputLocalPlayerSubsystem` self) "/Game/Input/Maps/IMC_Default.IMC_Default" 0 (struct)))

(event `EnhancedInput|/Game/Input/Actions/IA_Move`
  (params (ActionValue :type "Vector2D Structure") (ElapsedSeconds :type "Float (double-precision)") (TriggeredSeconds :type "Float (double-precision)") (InputAction :type "InputAction Object Reference" :default "/Game/Input/Actions/IA_Move.IA_Move"))
  (bind (_returnvalue_roll _returnvalue_pitch _returnvalue_yaw) (`KismetMathLibrary.BreakRotator` (`Pawn.GetControlRotation` (`self.As BP Ballisfaction Player`))))
  (:`Triggered`
    (`PrimitiveComponent.AddForce` (`/Game/Blueprints/Player/BP_BallisfactionPlayer.StaticMesh` (`self.As BP Ballisfaction Player`)) (* (`KismetMathLibrary.GreaterGreater_VectorRotator` (`KismetMathLibrary.Conv_Vector2DToVector` ActionValue) (`KismetMathLibrary.MakeRotator` 0.0 0.0 _returnvalue_yaw)) 100000.0) "None" false)))

(fn `UserConstructionScript`)