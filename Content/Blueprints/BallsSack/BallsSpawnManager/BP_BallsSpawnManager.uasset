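; BP_BallsSpawnManager keeps balls launching from the level's BP_BallsSack actors, up to a maximum live count.
; On BeginPlay it gathers every sack and starts a looping timer that asks each in turn to launch a ball until the cap is reached.
; It tracks each launched ball and binds to its destroyed event, with a BallDestroyed handler that removes balls from the tracked list.
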(event `self.ReceiveBeginPlay`
  (bind _outactors (`GameplayStatics.GetAllActorsOfClass` "/Game/Blueprints/BallsSack/BP_BallsSack.BP_BallsSack_C"))
  (set `self.BallsSacks` _outactors)
  (`KismetSystemLibrary.K2_SetTimer` null "InitiateBallsSpawn" 2.0 true false 1.0))

(event `BallDestroyed`
  (params (DestroyedBall :type "/Game/Blueprints/Balls/BP_Ball Object Reference"))
  (`KismetArrayLibrary.Array_RemoveItem` (`self.SpawnedBalls`) DestroyedBall))

(fn `InitiateBallsSpawn`
  (for _array_element (`self.BallsSacks`)
    (if (== (`KismetArrayLibrary.Array_Length` (`self.SpawnedBalls`)) (`self.MaxSpawnedBallsAmmount`))
      (break)
      (else
        (bind _spawnedball (`/Game/Blueprints/BallsSack/BP_BallsSack.LaunchBall` _array_element))
        (add `/Game/Blueprints/Balls/BP_Ball.OnBallDestroyed` _spawnedball (`|CreateDelegate` :!event `BallDestroyed`))
        (`KismetArrayLibrary.Array_Add` (`self.SpawnedBalls`) _spawnedball)))))

(fn `UserConstructionScript`)