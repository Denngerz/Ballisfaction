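; BP_Ball is the ball actor in Ballisfaction that knocks bricks loose and keeps the game mode's ball count updated.
; It registers with BallisfactionGameMode on BeginPlay and deregisters when destroyed, printing a debug string if either cast fails.
; When its capsule stops overlapping a BP_Brick, it enables physics simulation on that brick's cube and activates the brick's explosion component.
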(event `self.ReceiveBeginPlay`
  (bind _asballisfaction_game_mode (cast `BallisfactionGameMode` (`GameplayStatics.GetGameMode`))
    (:`then`
      (`BallisfactionGameMode.AddNewBall` _asballisfaction_game_mode))
    (:`CastFailed`
      (`KismetSystemLibrary.PrintString` "CAST TO BALLISFACTION_GAME_MODE"))))

(event `self.Capsule.OnComponentEndOverlap`
  (params (OverlappedComponent :type "PrimitiveComponent Object Reference") (OtherActor :type "Actor Object Reference") (OtherComp :type "PrimitiveComponent Object Reference") (OtherBodyIndex :type Integer))
  (bind _asbp_brick (cast `/Game/Blueprints/Bricks/BP_Brick` OtherActor))
  (`PrimitiveComponent.SetSimulatePhysics` (`/Game/Blueprints/Bricks/BP_Brick.Cube` _asbp_brick) true)
  (`ActorComponent.Activate` (`/Game/Blueprints/Bricks/BP_Brick.P_ky_explosion` _asbp_brick) false))

(event `self.ReceiveDestroyed`
  (bind _asballisfaction_game_mode (cast `BallisfactionGameMode` (`GameplayStatics.GetGameMode`))
    (:`then`
      (`BallisfactionGameMode.RemoveExistingBall` _asballisfaction_game_mode)
      (`self.K2_DestroyActor`))
    (:`CastFailed`
      (`KismetSystemLibrary.PrintString` "CAST TO BALLISFACTION_GAME_MODE"))))

(fn `UserConstructionScript`)