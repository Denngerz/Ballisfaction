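; BP_BallisfactionPlayer is the player Blueprint, turning movement and rotation input into physics forces on its static mesh.
; Move input is rotated by control yaw and applied as a force, while the X component of rotation input becomes torque around the Z axis.
; Both are multiplied by a fixed strength and a gameplay attribute value read from the Ballisfaction ability system.
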(event `/Game/Ballisfaction/Interfaces/BPI_Movable.ProccessMoveInput`
  (params (Direction :type "Vector Structure"))
  (bind (_returnvalue_roll _returnvalue_pitch _returnvalue_yaw) (`KismetMathLibrary.BreakRotator` (`self.GetControlRotation`)))
  (`PrimitiveComponent.AddForce` (`self.StaticMesh`) (* (`KismetMathLibrary.GreaterGreater_VectorRotator` Direction (`KismetMathLibrary.MakeRotator` 0.0 0.0 _returnvalue_yaw)) 5000.0 (`.ReturnValue` (`AbilitySystemComponent.GetGameplayAttributeValue` (`self.BallisfactionAbilitySystem`) (struct :`AttributeName` "Speed" :`Attribute` "/Script/BallisfactionProject.MovementSet:Speed" :`AttributeOwner` "/Script/CoreUObject.Class'/Script/BallisfactionProject.MovementSet'")))) "None" false))

(event `/Game/Ballisfaction/Interfaces/BPI_Rotatable.ProccessRotationInput`
  (params (Direction :type "Vector Structure"))
  (`PrimitiveComponent.AddTorqueInDegrees` (`self.StaticMesh`) (`KismetMathLibrary.MakeVector` 0.0 0.0 (* (.x Direction) 10000000.0 (`.ReturnValue` (`AbilitySystemComponent.GetGameplayAttributeValue` (`self.BallisfactionAbilitySystem`) (struct :`AttributeName` "RotationSpeed" :`Attribute` "/Script/BallisfactionProject.MovementSet:RotationSpeed" :`AttributeOwner` "/Script/CoreUObject.Class'/Script/BallisfactionProject.MovementSet'"))))) "None" false))

(fn `UserConstructionScript`)