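; BP_MatryoshkaBall is a ball that breaks into resized copies of itself when it hits something fast enough.
; It extends the parent's hit handling, checking the mesh's velocity against a split speed threshold.
; A loop spawns copies at its transform, scales their meshes by a size multiplier, and destroys the original within the loop body.
; Copies spawn with splitting disabled, so the split happens only one generation deep.
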(fn `ProccessActorHit`
  (params (HitActor :type "Actor Object Reference"))
  (locals (SizeMultiplier :type "Float (double-precision)" :default 0.7))
  (bind (_returnvalue_location _returnvalue_rotation) (`KismetMathLibrary.BreakTransform` (`self.GetTransform`)))
  (`parent.ProccessActorHit` HitActor)
  (if (`self.ShouldSplit`)
    (if (>= (`KismetMathLibrary.VSize` (`SceneComponent.GetComponentVelocity` (`self.StaticMesh`))) (`self.SpeedToSplit`))
      (for _ (range 2)
        (bind _returnvalue (`|SpawnActorFromClass` "BP_MatryoshkaBall_C" (`KismetMathLibrary.MakeTransform` _returnvalue_location _returnvalue_rotation) "Undefined" "MultiplyWithRoot" null false null))
        (bind _staticmesh (`BallisfactionBall.StaticMesh` _returnvalue))
        (`SceneComponent.SetWorldScale3D` _staticmesh (* (`SceneComponent.K2_GetComponentScale` _staticmesh) (`local.SizeMultiplier`)))
        (`self.K2_DestroyActor`)))))

(fn `UserConstructionScript`
  (`parent.UserConstructionScript`))