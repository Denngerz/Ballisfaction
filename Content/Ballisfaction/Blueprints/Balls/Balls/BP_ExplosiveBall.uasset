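; Explosive ball variant that deals area damage to bricks on high-speed impacts.
; ProccessActorHit override: at or above ExplosionSpeed, hitting a BP_Brick triggers a debug-drawn sphere trace around the ball; slower hits use parent handling.
; Traced bricks receive GE_ExplosionDamage through their own Ability System Component, with negated GetPotentialDamage passed as a SetByCaller magnitude.
; Fast hits on non-bricks do nothing and skip parent handling.
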(fn `ProccessActorHit`
  (params (HitActor :type "Actor Object Reference"))
  (locals (Damage :type "Float (single-precision)" :default 0.0))
  (bind _returnvalue (`self.K2_GetActorLocation`))
  (if (>= (`KismetMathLibrary.VSize` (`self.GetVelocity`)) (`self.ExplosionSpeed`))
    (cast `/Game/Ballisfaction/Blueprints/Bricks/BP_Brick` HitActor)
    (bind _returnvalue_2 (`self.GetPotentialDamage`))
    (set `local.Damage` _returnvalue_2)
    (bind _outhits (`KismetSystemLibrary.SphereTraceMulti` :`Start` _returnvalue :`End` _returnvalue :`Radius` 200.0 :`TraceChannel` "TraceTypeQuery1" :`DrawDebugType` "ForDuration" :`DrawTime` 2.0))
    (for _array_element _outhits
      (bind _asbp_brick (cast `/Game/Ballisfaction/Blueprints/Bricks/BP_Brick` (`.HitActor` (`GameplayStatics.BreakHitResult` _array_element))))
      (bind _returnvalue_3 (`AbilitySystemBlueprintLibrary.GetAbilitySystemComponent` _asbp_brick))
      (`/Engine/EditorBlueprintResources/StandardMacros.IsValid` _returnvalue_3
        (:`Is Valid`
          (bind _returnvalue_4 (`AbilitySystemBlueprintLibrary.AssignTagSetByCallerMagnitude` (`AbilitySystemComponent.MakeOutgoingSpec` :`self` _returnvalue_3 :`GameplayEffectClass` "/Game/Ballisfaction/Blueprints/Abilities/BallsAbilities/GE_ExplosionDamage.GE_ExplosionDamage_C") (struct :`TagName` "Data.Damage.Magnitude") (* (`local.Damage`) -1.0)))
          (`AbilitySystemComponent.BP_ApplyGameplayEffectSpecToSelf` _returnvalue_3 _returnvalue_4))))
    (else
      (`parent.ProccessActorHit` HitActor))))

(fn `UserConstructionScript`
  (`parent.UserConstructionScript`))