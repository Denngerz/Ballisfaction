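; BP_Ball is the physics ball in Ballisfaction that damages bricks it hits and registers itself with the game mode's ball count.
; Each hit clamps velocity to MaxBallSpeed, updates a contact timer on player contact, then processes brick impacts.
; Brick hits trigger the brick's explosion effect and apply GE_BallDamage through GAS, passing negated potential damage as a SetByCaller magnitude.
; DestroySelf removes the ball from the game mode's count.
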(event `self.StaticMesh.OnComponentHit`
  (params (HitComponent :type "PrimitiveComponent Object Reference") (OtherActor :type "Actor Object Reference") (OtherComp :type "PrimitiveComponent Object Reference") (NormalImpulse :type "Vector Structure") (Hit :type "HitResult Structure (by ref)"))
  (`|ExecutionSequence`
    (:`then_0`
      (`self.HandleSpeedAfterHit`))
    (:`then_1`
      (cast `/Game/Ballisfaction/Blueprints/Player/BP_BallisfactionPlayer` OtherActor)
      (`self.UpdateContactTimer`))
    (:`then_2`
      (`self.ProccessActorHit` OtherActor))))

(event `self.ReceiveBeginPlay`
  (bind _asballisfaction_game_mode (cast `BallisfactionGameMode` (`GameplayStatics.GetGameMode`))
    (:`then`
      (`BallisfactionGameMode.AddNewBall` _asballisfaction_game_mode))
    (:`CastFailed`
      (`KismetSystemLibrary.PrintString` "CAST TO BALLISFACTION_GAME_MODE"))))

(event `self.DestroySelf`
  (bind _asballisfaction_game_mode (cast `BallisfactionGameMode` (`GameplayStatics.GetGameMode`))
    (:`then`
      (`BallisfactionGameMode.RemoveExistingBall` _asballisfaction_game_mode))
    (:`CastFailed`
      (`KismetSystemLibrary.PrintString` "CAST TO BALLISFACTION_GAME_MODE"))))

(fn `HandleSpeedAfterHit`
  (bind _returnvalue (`SceneComponent.GetComponentVelocity` (`self.StaticMesh`)))
  (if (> (`KismetMathLibrary.VSize` _returnvalue) (`self.MaxBallSpeed`))
    (`PrimitiveComponent.SetAllPhysicsLinearVelocity` (`self.StaticMesh`) (* (`KismetMathLibrary.Normal` _returnvalue) (`self.MaxBallSpeed`)) false)))

(fn `ProccessActorHit`
  (params (HitActor :type "Actor Object Reference"))
  (bind _asbp_brick (cast `/Game/Ballisfaction/Blueprints/Bricks/BP_Brick` HitActor))
  (`ActorComponent.Activate` (`/Game/Ballisfaction/Blueprints/Bricks/BP_Brick.P_ky_explosion` _asbp_brick) false)
  (bind _returnvalue (`AbilitySystemBlueprintLibrary.GetAbilitySystemComponent` _asbp_brick))
  (`/Engine/EditorBlueprintResources/StandardMacros.IsValid` _returnvalue
    (:`Is Valid`
      (bind _returnvalue_2 (`self.GetPotentialDamage`))
      (bind _returnvalue_3 (`AbilitySystemBlueprintLibrary.AssignTagSetByCallerMagnitude` (`AbilitySystemComponent.MakeOutgoingSpec` :`self` _returnvalue :`GameplayEffectClass` "/Game/Ballisfaction/Blueprints/Abilities/GE_BallDamage.GE_BallDamage_C") (struct :`TagName` "Damage.Ball") (* _returnvalue_2 -1.0)))
      (`AbilitySystemComponent.BP_ApplyGameplayEffectSpecToSelf` _returnvalue _returnvalue_3))))

(fn `UserConstructionScript`)