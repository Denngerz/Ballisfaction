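; Gameplay ability for player sprinting, active while the input is held and its cost is affordable.
; On press, an attribute ratio above 20% applies GE_Sprint and clears stamina regeneration abilities, otherwise the ability cancels.
; A fast looping timer drives repeated cost commits, ending the ability when unaffordable.
; Input release also ends it, and a non-cancelled end removes the effect and grants and activates GA_StaminaRegeneration once.
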(event `self.K2_ActivateAbility`
  (bind _returnvalue (`AbilitySystemBlueprintLibrary.GetAbilitySystemComponent` (`self.GetAvatarActorFromActorInfo`)))
  (bind _returnvalue_2 (`AbilitySystemBlueprintLibrary.GetAbilitySystemComponent` (`self.GetAvatarActorFromActorInfo`)))
  (`AbilityTask_WaitInputPress.WaitInputPress` false
    (:`then`
      (`AbilityTask_WaitInputRelease.WaitInputRelease` false
        (:`OnRelease`
          (`self.K2_EndAbility`))))
    (:`OnPress`
      (if (> (/ (`.ReturnValue` (`AbilitySystemComponent.GetGameplayAttributeValue` _returnvalue (struct :`AttributeName` "StaminaPoints" :`Attribute` "/Script/BallisfactionProject.StaminaSet:StaminaPoints" :`AttributeOwner` "/Script/CoreUObject.Class'/Script/BallisfactionProject.StaminaSet'"))) (`.ReturnValue` (`AbilitySystemComponent.GetGameplayAttributeValue` _returnvalue (struct :`AttributeName` "MaxStaminaPoints" :`Attribute` "/Script/BallisfactionProject.StaminaSet:MaxStaminaPoints" :`AttributeOwner` "/Script/CoreUObject.Class'/Script/BallisfactionProject.StaminaSet'")))) 0.2)
        (bind _returnvalue_3 (`self.BP_ApplyGameplayEffectToOwner` "/Game/Ballisfaction/Blueprints/Abilities/PlayerAbilities/Sprint/GE_Sprint.GE_Sprint_C"))
        (set `self.SprintEffect` _returnvalue_3)
        (`KismetSystemLibrary.K2_SetTimerDelegate` (`|CreateDelegate` :!event `ApplySprintCost`) 0.01 true)
        (bind _outabilityhandles (`AbilitySystemComponent.FindAllAbilitiesWithTags` _returnvalue_2 (struct :`GameplayTags` (struct :`(TagName` "Ability.Status.StaminaRegeneration"))) true))
        (for _array_element _outabilityhandles
          (`AbilitySystemComponent.ClearAbility` _returnvalue_2 _array_element))
        (else
          (`self.K2_CancelAbility`))))))

(event `self.K2_OnEndAbility`
  (params (bWasCancelled :type Boolean))
  (if (not bWasCancelled)
    (`self.BP_RemoveGameplayEffectFromOwnerWithHandle` (`self.SprintEffect`))
    (`AbilitySystemComponent.K2_GiveAbilityAndActivateOnce` (`AbilitySystemBlueprintLibrary.GetAbilitySystemComponent` (`self.GetAvatarActorFromActorInfo`)) "/Game/Ballisfaction/Blueprints/Abilities/PlayerAbilities/Statuses/StaminaRegeneration/GA_StaminaRegeneration.GA_StaminaRegeneration_C" 0 -1)))

(event `ApplySprintCost`
  (`self.K2_CommitAbilityCost` false)
  (bind _returnvalue (`self.K2_CheckAbilityCost`))
  (if (not _returnvalue)
    (`self.K2_EndAbility`)))