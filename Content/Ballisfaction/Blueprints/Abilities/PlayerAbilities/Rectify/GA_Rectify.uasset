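; GA_Rectify is a player Gameplay Ability that spends stamina to rotate the player's physics mesh toward 90-degree world yaw.
; A press above a 20% attribute ratio starts fast looping timers for correction and cost, and clears stamina regeneration abilities.
; Correction raises angular damping and applies torque scaled by yaw error and an attribute.
; Release or unaffordable cost restores damping and ends the ability, which re-grants GA_StaminaRegeneration.
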(event `self.K2_ActivateAbility`
  (bind _returnvalue (`AbilitySystemBlueprintLibrary.GetAbilitySystemComponent` (`self.GetAvatarActorFromActorInfo`)))
  (bind _returnvalue_2 (`AbilitySystemBlueprintLibrary.GetAbilitySystemComponent` (`self.GetAvatarActorFromActorInfo`)))
  (bind _asbp_ballisfaction_player (cast `/Game/Ballisfaction/Blueprints/Player/BP_BallisfactionPlayer` (`self.GetAvatarActorFromActorInfo`)))
  (set `self.OwnerStaticMesh` (`/Game/Ballisfaction/Blueprints/Player/BP_BallisfactionPlayer.StaticMesh` _asbp_ballisfaction_player))
  (`AbilityTask_WaitInputPress.WaitInputPress` false
    (:`then`
      (`AbilityTask_WaitInputRelease.WaitInputRelease` false
        (:`OnRelease`
          (`PrimitiveComponent.SetAngularDamping` (`self.OwnerStaticMesh`) 3.0)
          (`self.K2_EndAbility`))))
    (:`OnPress`
      (if (> (/ (`.ReturnValue` (`AbilitySystemComponent.GetGameplayAttributeValue` _returnvalue (struct :`AttributeName` "StaminaPoints" :`Attribute` "/Script/BallisfactionProject.StaminaSet:StaminaPoints" :`AttributeOwner` "/Script/CoreUObject.Class'/Script/BallisfactionProject.StaminaSet'"))) (`.ReturnValue` (`AbilitySystemComponent.GetGameplayAttributeValue` _returnvalue (struct :`AttributeName` "MaxStaminaPoints" :`Attribute` "/Script/BallisfactionProject.StaminaSet:MaxStaminaPoints" :`AttributeOwner` "/Script/CoreUObject.Class'/Script/BallisfactionProject.StaminaSet'")))) 0.2)
        (`KismetSystemLibrary.K2_SetTimerDelegate` (`|CreateDelegate` :!event `Rectify`) 0.01 true)
        (`self.K2_CommitAbilityCost` false)
        (`KismetSystemLibrary.K2_SetTimerDelegate` (`|CreateDelegate` :!event `ApplyStaminaCost`) 0.01 true)
        (bind _outabilityhandles (`AbilitySystemComponent.FindAllAbilitiesWithTags` _returnvalue_2 (struct :`GameplayTags` (struct :`(TagName` "Ability.Status.StaminaRegeneration"))) true))
        (for _array_element _outabilityhandles
          (`AbilitySystemComponent.ClearAbility` _returnvalue_2 _array_element))
        (else
          (`self.K2_CancelAbility`))))))

(event `Rectify`
  (bind _ownerstaticmesh (`self.OwnerStaticMesh`))
  (bind (_returnvalue_roll _returnvalue_pitch _returnvalue_yaw) (`KismetMathLibrary.BreakRotator` (`SceneComponent.K2_GetComponentRotation` _ownerstaticmesh)))
  (bind _returnvalue (`self.K2_CheckAbilityCost`))
  (if _returnvalue
    (`PrimitiveComponent.SetAngularDamping` _ownerstaticmesh 20.0)
    (`PrimitiveComponent.AddTorqueInDegrees` (`self.OwnerStaticMesh`) (`KismetMathLibrary.MakeVector` 0.0 0.0 (* (`KismetMathLibrary.NormalizeAxis` (- 90.0 _returnvalue_yaw)) 10000000.0 (`.ReturnValue` (`AbilitySystemComponent.GetGameplayAttributeValue` (`AbilitySystemBlueprintLibrary.GetAbilitySystemComponent` (`self.GetAvatarActorFromActorInfo`)) (struct :`AttributeName` "RotationSpeed" :`Attribute` "/Script/BallisfactionProject.MovementSet:RotationSpeed" :`AttributeOwner` "/Script/CoreUObject.Class'/Script/BallisfactionProject.MovementSet'"))))) "None" false)
    (else
      (`PrimitiveComponent.SetAngularDamping` (`self.OwnerStaticMesh`) 3.0)
      (`self.K2_EndAbility`))))

(event `ApplyStaminaCost`
  (`self.K2_CommitAbilityCost` false))

(event `self.K2_OnEndAbility`
  (params (bWasCancelled :type Boolean))
  (`AbilitySystemComponent.K2_GiveAbilityAndActivateOnce` (`AbilitySystemBlueprintLibrary.GetAbilitySystemComponent` (`self.GetAvatarActorFromActorInfo`)) "/Game/Ballisfaction/Blueprints/Abilities/PlayerAbilities/Statuses/StaminaRegeneration/GA_StaminaRegeneration.GA_StaminaRegeneration_C" 0 -1))