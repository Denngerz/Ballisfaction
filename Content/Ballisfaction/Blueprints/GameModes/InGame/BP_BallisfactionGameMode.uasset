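; BP_BallisfactionGameMode is the in-game game mode for Ballisfaction, handling scoring outcomes and the end of a game.
; UpdateScore adds a point to the first player's BP_BallisfactionPlayerState on a score, otherwise applying GE_PureHealthDamage to that player's pawn through the Gameplay Ability System.
; OnEndGame waits briefly, then loads the main menu level.
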(event `UpdateScore`
  (params (PlayerScored :type Boolean))
  (if PlayerScored
    (bind _asbp_ballisfaction_player_state (cast `/Game/Ballisfaction/Blueprints/PlayerState/BP_BallisfactionPlayerState` (`GameplayStatics.GetPlayerState` 0)))
    (`BallisfactionPlayerState.AddPointsToScore` _asbp_ballisfaction_player_state 1.0)
    (else
      (bind _asbp_ballisfaction_player (cast `/Game/Ballisfaction/Blueprints/Player/BP_BallisfactionPlayer` (`GameplayStatics.GetPlayerPawn` 0)))
      (`AbilitySystemComponent.BP_ApplyGameplayEffectToSelf` :`self` (`AbilitySystemBlueprintLibrary.GetAbilitySystemComponent` _asbp_ballisfaction_player) :`GameplayEffectClass` "/Game/Ballisfaction/Blueprints/Abilities/GE_PureHealthDamage.GE_PureHealthDamage_C"))))

(event `OnEndGame`
  (`KismetSystemLibrary.Delay` 3.0)
  (`GameplayStatics.OpenLevel` "L_MainMenu"))

(fn `UserConstructionScript`)