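; BP_BallsSack is a ball launcher that spawns BP_Ball actors into the game and shoots them out.
; BeginPlay starts a looping one-second timer, alongside a LaunchBall event that asks BallisfactionGameMode whether another ball may spawn.
; When allowed, LaunchBall spawns a ball at the Scene component's location and applies a large force to its mesh along the Arrow's forward vector.
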(event `self.ReceiveBeginPlay`
  (`KismetSystemLibrary.K2_SetTimerDelegate` (`|CreateDelegate` :!event `LaunchBall`) 1.0 true false 1.0))

(event `LaunchBall`
  (bind _asballisfaction_game_mode (cast `BallisfactionGameMode` (`GameplayStatics.GetGameMode`)))
  (bind _returnvalue (`BallisfactionGameMode.CanSpawnNewBall` _asballisfaction_game_mode))
  (if _returnvalue
    (bind _returnvalue_2 (`|SpawnActorFromClass` "/Game/Ballisfaction/Blueprints/Balls/BP_Ball.BP_Ball_C" (`KismetMathLibrary.MakeTransform` (`SceneComponent.K2_GetComponentLocation` (`self.Scene`))) "Undefined" "MultiplyWithRoot" null null))
    (`PrimitiveComponent.AddForce` (`BallisfactionBall.StaticMesh` _returnvalue_2) (* (* (`SceneComponent.GetForwardVector` (`self.Arrow`)) 50000.0) 5.0) "None" false)))

(fn `UserConstructionScript`)