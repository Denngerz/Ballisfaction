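; BP_BrickLegend_test is a test brick Blueprint for Ballisfaction that breaks away when it runs out of health.
; On BeginPlay it binds a handler to its HealthComponent's out-of-health event.
; That handler sets the cube to query-only collision and enables physics simulation.
; After a delay it fires the brick-destroyed dispatcher and destroys the actor.
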(event `self.ReceiveBeginPlay`
  (add `BallisfactionHealthComponent.OnOutOfHealth` (`self.HealthComponent`) (`|CreateDelegate` :!event `OnOutOfHealth`)))

(event `OnOutOfHealth`
  (`PrimitiveComponent.SetCollisionEnabled` (`self.Cube`) "QueryOnly")
  (`PrimitiveComponent.SetSimulatePhysics` (`self.Cube`) true)
  (`KismetSystemLibrary.Delay` 6.0)
  (`self.OnBrickDestroyed`)
  (`self.K2_DestroyActor`))

(fn `UserConstructionScript`)