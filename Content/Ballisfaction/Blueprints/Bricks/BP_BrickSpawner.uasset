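; BP_BrickSpawner is a placeable actor that keeps one brick of a configurable class present at its location.
; On BeginPlay it spawns the brick at its own transform and stores the reference.
; A looping ten-second timer checks whether that brick is still valid and respawns it at the same spot once it has been destroyed.
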(event `self.ReceiveBeginPlay`
  ; Nakakav
  (`self.SpawnBrick`)
  (`KismetSystemLibrary.K2_SetTimer` null "CheckbrickDestroyed" 10.0 true))

(fn `CheckbrickDestroyed`
  (`/Engine/EditorBlueprintResources/StandardMacros.IsValid` (`self.SpawnedBrick `)
    (:`Is Not Valid`
      (`self.SpawnBrick`))))

(fn `SpawnBrick`
  (bind _returnvalue (`|SpawnActorFromClass` (`self.BrickClassToSpawn`) (`self.GetTransform`) "Undefined" "MultiplyWithRoot" null null))
  (set `self.SpawnedBrick ` _returnvalue))

(fn `UserConstructionScript`)