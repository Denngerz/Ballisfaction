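; BP_BrickGrid is an actor that builds and tears down the grid of brick holders for each Ballisfaction round.
; It binds to the game mode's round start and end events on BeginPlay.
; On round start it spawns evenly spaced BP_BrickHolder actors from its own location, with the row count from the game mode and a fixed column count.
; On round end it destroys the stored holders without clearing the array.
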(event `self.ReceiveBeginPlay`
  (bind _asbp_ballisfaction_game_mode (cast `/Game/Ballisfaction/Blueprints/GameModes/InGame/BP_BallisfactionGameMode` (`GameplayStatics.GetGameMode`)))
  (add `BallisfactionGameMode.OnRoundStart` _asbp_ballisfaction_game_mode (`|CreateDelegate` :!event `OnRoundStart`))
  (add `BallisfactionGameMode.OnRoundEnd` _asbp_ballisfaction_game_mode (`|CreateDelegate` :!event `OnRoundEnd`)))

(event `self.SpawnHolders`
  (params (Rows :type Integer) (Columns :type Integer))
  (bind (_returnvalue_x _returnvalue_y _returnvalue_z) (`KismetMathLibrary.BreakVector` (`self.K2_GetActorLocation`)))
  (set `self.DeltaX` 0.0)
  (for _ (range 1 (+ Rows 1))
    (set `self.DeltaY` 0.0)
    (for _ (range 1 (+ Columns 1))
      (bind _returnvalue (`|SpawnActorFromClass` "/Game/Ballisfaction/Blueprints/Bricks/BP_BrickHolder.BP_BrickHolder_C" (`KismetMathLibrary.MakeTransform` (`KismetMathLibrary.MakeVector` (+ _returnvalue_x (`self.DeltaX`)) (+ _returnvalue_y (`self.DeltaY`)) _returnvalue_z)) "Undefined" "MultiplyWithRoot" null null))
      (`KismetArrayLibrary.Array_Add` (`self.BrickHolders`) _returnvalue)
      (set `self.DeltaY` (+ (`self.DeltaY`) 130.0)))
    (set `self.DeltaX` (+ (`self.DeltaX`) 130.0))))

(event `OnRoundStart`
  (bind _asbp_ballisfaction_game_mode (cast `/Game/Ballisfaction/Blueprints/GameModes/InGame/BP_BallisfactionGameMode` (`GameplayStatics.GetGameMode`)))
  (bind _returnvalue (`BallisfactionGameMode.GetBrickRowsAmount` _asbp_ballisfaction_game_mode))
  (`self.SpawnHolders` _returnvalue 13))

(event `OnRoundEnd`
  (`self.DestroyHolders`))

(event `DestroyHolders`
  (for _array_element (`self.BrickHolders`)
    (`self.K2_DestroyActor` _array_element)))

(fn `UserConstructionScript`)