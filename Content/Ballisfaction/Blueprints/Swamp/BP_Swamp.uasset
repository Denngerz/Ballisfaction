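; BP_Swamp is a short-lived slowing area that destroys itself on a timer roughly four seconds after spawning.
; Players entering its capsule receive the GE_SlowDown gameplay effect with a set-by-caller magnitude, removed on exit or swamp destruction through a stored handle.
; Other non-owner actors implementing BPI_Slowable get a slow-down message, with no matching restore here.
; Only one player reference and effect handle are stored at a time.
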(event `self.ReceiveBeginPlay`
  (`KismetSystemLibrary.K2_SetTimer` null "DestroySelf" 0.1 true false 4.0))

(event `self.Capsule.OnComponentBeginOverlap`
  (params (OverlappedComponent :type "PrimitiveComponent Object Reference") (OtherActor :type "Actor Object Reference") (OtherComp :type "PrimitiveComponent Object Reference") (OtherBodyIndex :type Integer) (bFromSweep :type Boolean) (SweepResult :type "HitResult Structure (by ref)"))
  (bind _asbp_ballisfaction_player (cast `/Game/Ballisfaction/Blueprints/Player/BP_BallisfactionPlayer` OtherActor)
    (:`then`
      (bind _output_get (set `self.PlayerRef` _asbp_ballisfaction_player))
      (bind _ballisfactionabilitysystemcomponent (`BallisfactionPlayer.BallisfactionAbilitySystemComponent` _output_get))
      (bind _returnvalue (`AbilitySystemBlueprintLibrary.AssignTagSetByCallerMagnitude` (`AbilitySystemComponent.MakeOutgoingSpec` :`self` _ballisfactionabilitysystemcomponent :`GameplayEffectClass` "/Game/Ballisfaction/Blueprints/Abilities/PlayerAbilities/SlowDown/GE_SlowDown.GE_SlowDown_C") (struct :`TagName` "Data.Movement.Slow.Magnitude") (`self.SpeedMultiplier`)))
      (bind _returnvalue_2 (`AbilitySystemComponent.BP_ApplyGameplayEffectSpecToSelf` _ballisfactionabilitysystemcomponent _returnvalue))
      (set `self.EffectOnPlayerHandle` _returnvalue_2))
    (:`CastFailed`
      (if (!= (`self.GetOwner`) OtherActor)
        (if (`KismetSystemLibrary.DoesImplementInterface` OtherActor "/Game/Ballisfaction/Interfaces/BPI_Slowable.BPI_Slowable_C")
          (message `/Game/Ballisfaction/Interfaces/BPI_Slowable.SlowDownActor` OtherActor (`self.SpeedMultiplier`)))))))

(event `self.Capsule.OnComponentEndOverlap`
  (params (OverlappedComponent :type "PrimitiveComponent Object Reference") (OtherActor :type "Actor Object Reference") (OtherComp :type "PrimitiveComponent Object Reference") (OtherBodyIndex :type Integer))
  (bind _playerref (`self.PlayerRef`))
  (`/Engine/EditorBlueprintResources/StandardMacros.IsValid` _playerref
    (:`Is Valid`
      (if (== _playerref OtherActor)
        (`AbilitySystemComponent.RemoveActiveGameplayEffect` (`BallisfactionPlayer.BallisfactionAbilitySystemComponent` (`self.PlayerRef`)) (`self.EffectOnPlayerHandle`) -1)))))

(event `self.ReceiveDestroyed`
  (bind _playerref (`self.PlayerRef`))
  (`/Engine/EditorBlueprintResources/StandardMacros.IsValid` _playerref
    (:`Is Valid`
      (`AbilitySystemComponent.RemoveActiveGameplayEffect` (`BallisfactionPlayer.BallisfactionAbilitySystemComponent` _playerref) (`self.EffectOnPlayerHandle`) -1))))

(fn `DestroySelf`
  (`self.K2_DestroyActor`))

(fn `UserConstructionScript`)