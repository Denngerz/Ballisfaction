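; Player controller for Ballisfaction that turns Enhanced Input into pawn movement, rotation and ability activation.
; On possess it caches the pawn and its ability system, sets game-only input and adds the default mapping context.
; Move and rotate reach the pawn through Movable and Rotatable interfaces, while Sprint and Rectify send press and release gameplay tags to the ability system.
; It also binds to the HUD's initialization event and can open the game HUD.
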(event `self.ReceiveBeginPlay`
  (bind _asbp_ballisfaction_hud (cast `/Game/Ballisfaction/Blueprints/HUD/BP_BallisfactionHUD` (`self.GetHUD`)))
  (bind _output_get (set `self.HUDLayout` _asbp_ballisfaction_hud))
  (add `BallisfactionHUD.OnInitializationComplited` _output_get (`|CreateDelegate` :!event `OpenGameHUD`)))

(event `self.ReceivePossess`
  (params (PossessedPawn :type "Pawn Object Reference"))
  (bind _output_get (set `self.Possessed Pawn` PossessedPawn))
  (bind _asballisfaction_ability_system (cast `BallisfactionAbilitySystem` (`AbilitySystemBlueprintLibrary.GetAbilitySystemComponent` _output_get)))
  (set `self.PawnsAbilitySystem` _asballisfaction_ability_system)
  (`WidgetBlueprintLibrary.SetInputMode_GameOnly` self)
  (message `EnhancedInputSubsystemInterface.AddMappingContext` (pcsubsystem `EnhancedInputLocalPlayerSubsystem` self) "/Game/Ballisfaction/Input/Mappings/IMC_Default.IMC_Default" 0 (struct)))

(event `EnhancedInput|/Game/Ballisfaction/Input/Actions/IA_Move`
  (params (ActionValue :type "Vector2D Structure") (ElapsedSeconds :type "Float (double-precision)") (TriggeredSeconds :type "Float (double-precision)") (InputAction :type "InputAction Object Reference" :default "/Game/Ballisfaction/Input/Actions/IA_Move.IA_Move"))
  (bind _possessed_pawn (`self.Possessed Pawn`))
  (:`Triggered`
    (`/Engine/EditorBlueprintResources/StandardMacros.IsValid` _possessed_pawn
      (:`Is Valid`
        (if (`KismetSystemLibrary.DoesImplementInterface` _possessed_pawn "/Game/Ballisfaction/Interfaces/BPI_Movable.BPI_Movable_C")
          (message `/Game/Ballisfaction/Interfaces/BPI_Movable.ProccessMoveInput` _possessed_pawn (`KismetMathLibrary.Conv_Vector2DToVector` ActionValue)))))))

(event `EnhancedInput|/Game/Ballisfaction/Input/Actions/IA_Rotate`
  (params (ActionValue :type "Vector2D Structure") (ElapsedSeconds :type "Float (double-precision)") (TriggeredSeconds :type "Float (double-precision)") (InputAction :type "InputAction Object Reference" :default "/Game/Ballisfaction/Input/Actions/IA_Rotate.IA_Rotate"))
  (bind _possessed_pawn (`self.Possessed Pawn`))
  (:`Triggered`
    (`/Engine/EditorBlueprintResources/StandardMacros.IsValid` null
      (:`Is Valid`
        (if (`KismetSystemLibrary.DoesImplementInterface` _possessed_pawn "/Game/Ballisfaction/Interfaces/BPI_Rotatable.BPI_Rotatable_C")
          (message `/Game/Ballisfaction/Interfaces/BPI_Rotatable.ProccessRotationInput` _possessed_pawn (`KismetMathLibrary.Conv_Vector2DToVector` ActionValue)))))))

(event `EnhancedInput|/Game/Ballisfaction/Input/Actions/IA_Sprint`
  (params (ActionValue :type Boolean) (ElapsedSeconds :type "Float (double-precision)") (TriggeredSeconds :type "Float (double-precision)") (InputAction :type "InputAction Object Reference" :default "/Game/Ballisfaction/Input/Actions/IA_Sprint.IA_Sprint"))
  (:`Started`
    (bind _pawnsabilitysystem (`self.PawnsAbilitySystem`)
      (:`then`
        (`BallisfactionAbilitySystem.AbilityInputTagPressed` _pawnsabilitysystem (struct :`TagName` "Ability.Sprint")))
      (:`else`)))
  (:`Completed`
    (bind _pawnsabilitysystem_2 (`self.PawnsAbilitySystem`)
      (:`then`
        (`BallisfactionAbilitySystem.AbilityInputTagReleased` _pawnsabilitysystem_2 (struct :`TagName` "Ability.Sprint")))
      (:`else`))))

(event `EnhancedInput|/Game/Ballisfaction/Input/Actions/IA_Rectify`
  (params (ActionValue :type Boolean) (ElapsedSeconds :type "Float (double-precision)") (TriggeredSeconds :type "Float (double-precision)") (InputAction :type "InputAction Object Reference" :default "/Game/Ballisfaction/Input/Actions/IA_Rectify.IA_Rectify"))
  (:`Started`
    (bind _pawnsabilitysystem (`self.PawnsAbilitySystem`)
      (:`then`
        (`BallisfactionAbilitySystem.AbilityInputTagPressed` _pawnsabilitysystem (struct :`TagName` "Ability.Rectify")))
      (:`else`)))
  (:`Completed`
    (bind _pawnsabilitysystem_2 (`self.PawnsAbilitySystem`)
      (:`then`
        (`BallisfactionAbilitySystem.AbilityInputTagReleased` _pawnsabilitysystem_2 (struct :`TagName` "Ability.Rectify")))
      (:`else`))))

(event `OpenGameHUD`
  (`/Game/Ballisfaction/Blueprints/HUD/BP_BallisfactionHUD.OpenGameHUD` (`self.HUDLayout`)))

(fn `UserConstructionScript`)