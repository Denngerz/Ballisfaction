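; BP_BallisfactionHUD is the Ballisfaction HUD Blueprint that opens the game's main UI screens.
; Events for the main menu, game HUD and end-of-round shop each cast the Layout widget to WBP_HUDLayout.
; Each then pushes its screen widget onto that layout's menu, game or modal stack respectively, keeping the UI in separate layers.
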(event `OpenMainMenu`
  (bind _aswbp_hudlayout (cast `/Game/Ballisfaction/CommonUI/Widgets/WBP_HUDLayout` (`self.Layout`)))
  (`/Game/Ballisfaction/CommonUI/Widgets/WBP_HUDLayout.PushToMenuStack` _aswbp_hudlayout "/Game/Ballisfaction/CommonUI/Widgets/MenuHUD/WBP_MainMenuHUD.WBP_MainMenuHUD_C"))

(event `OpenGameHUD`
  (bind _aswbp_hudlayout (cast `/Game/Ballisfaction/CommonUI/Widgets/WBP_HUDLayout` (`self.Layout`)))
  (`/Game/Ballisfaction/CommonUI/Widgets/WBP_HUDLayout.PushToGameStack` _aswbp_hudlayout "/Game/Ballisfaction/CommonUI/Widgets/GameHUD/WBP_GameHUD.WBP_GameHUD_C"))

(event `OpenShop`
  (bind _aswbp_hudlayout (cast `/Game/Ballisfaction/CommonUI/Widgets/WBP_HUDLayout` (`self.Layout`)))
  (`/Game/Ballisfaction/CommonUI/Widgets/WBP_HUDLayout.PushToModalStack` _aswbp_hudlayout "/Game/Ballisfaction/CommonUI/Widgets/GameHUD/EndRoundShop/WBP_EndRoundShop.WBP_EndRoundShop_C"))

(fn `UserConstructionScript`)